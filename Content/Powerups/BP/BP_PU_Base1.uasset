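; BP_PU_Base1 is a powerup Blueprint that heals the first player's pawn over ticks.
; On activation it hides its static mesh and destroys itself.
; Each powerup tick finds the SHealthComponent on player pawn 0 and calls Heal with a variable amount.
; The state-change event is empty, and a leftover SCharacter lookup loop is never run.
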(event EventOnPowerupStateChange
  (params (bNewIsActive :type Boolean)))

(event EventOnPowerupTicked
  (bind _returnvalue (Game|Player|GetPlayerPawn 0))
  (bind _returnvalue_2 (Actor|GetComponentbyClass _returnvalue "/Script/CoopGame.SHealthComponent"))
  (Utilities|IsValid _returnvalue_2
    (:Is%20Valid
      (Class|SHealthComponent|Heal _returnvalue_2 (Variables|Default|GetNewVar_0)))))

(event EventOnActivated
  (Rendering|SetVisibility (Variables|Default|GetStaticMesh) false true)
  (Actor|DestroyActor))

(fn ConstructionScript)